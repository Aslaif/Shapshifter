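; Player character for a 2D side-scroller: a Paper2D knight that runs, jumps and attacks using Enhanced Input, flipping via control rotation.
; Tick selects flipbooks from movement state and checks playback frames to time footstep sounds and attack hits, which destroy overlapping actors.
; Attacks start only when grounded, block move and jump input, and repeat while held.
; A timeline-driven material flash is triggered from BeginPlay after creating dynamic materials.
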(event `EnhancedInput|/Game/GameAssets/Input/Aktions/IA_Move`
  (params (ActionValue :type "Float (double-precision)") (ElapsedSeconds :type "Float (double-precision)") (TriggeredSeconds :type "Float (double-precision)") (InputAction :type "InputAction Object Reference" :default "/Game/GameAssets/Input/Aktions/IA_Move.IA_Move"))
  (:`Triggered`
    (if (not (`self.IsAttacking`))
      (`self.AddMovementInput` (1.0 0.0 0.0) ActionValue)
      ;[1 1 1] Flip Char
      (`Controller.SetControlRotation` (`self.GetController`) (select `bool` (> ActionValue 0.0) :`false` (`KismetMathLibrary.MakeRotator` 0.0 0.0 180.0) :`true` (`KismetMathLibrary.MakeRotator` 0.0))))))

(event `self.ReceiveBeginPlay`
  ;[1 1 1] Connect with InputMappingContext
  (bind _asplayer_controller (cast `PlayerController` (`self.GetController`)))
  (`EnhancedInputSubsystemInterface.AddMappingContext` (pcsubsystem `EnhancedInputLocalPlayerSubsystem` _asplayer_controller) "/Game/GameAssets/Input/IMC_SideScroller.IMC_SideScroller" 0 (struct))
  ;[1 1 1] Init dynamic material
  (for _array_element (`SceneComponent.GetChildrenComponents` (`self.Moon`) false)
    (bind _aspaper_sprite_component (cast `PaperSpriteComponent` _array_element))
    (bind _returnvalue (`PrimitiveComponent.CreateDynamicMaterialInstance` _aspaper_sprite_component 0 null "None"))
    (`KismetArrayLibrary.Array_Add` (`self.DynamicLayer`) _returnvalue)
    (bind _returnvalue_2 (`PrimitiveComponent.CreateDynamicMaterialInstance` (`self.Sprite`) 0 null "None"))
    (set `self.DynamicSpriteMaterial` _returnvalue_2)
    (`KismetSystemLibrary.Delay` 3.0)
    (`self.TriggerFlash` 1.0)))

(event `EnhancedInput|/Game/GameAssets/Input/Aktions/IA_Attack`
  (params (ActionValue :type Boolean) (ElapsedSeconds :type "Float (double-precision)") (TriggeredSeconds :type "Float (double-precision)") (InputAction :type "InputAction Object Reference" :default "/Game/GameAssets/Input/Aktions/IA_Attack.IA_Attack"))
  (:`Started`
    (set `self.IsAttackInput` true)
    (if (`NavMovementComponent.IsMovingOnGround` (`self.CharacterMovement`))
      (`PaperFlipbookComponent.SetFlipbook` (`self.Sprite`) "/Game/GameAssets/2DTestAsset/KnightAttack.KnightAttack")
      (set `self.IsAttacking` true)
      (`PaperFlipbookComponent.SetLooping` (`self.Sprite`) false)))
  (:`Completed`
    (set `self.IsAttackInput` false)))

(event `EnhancedInput|/Game/GameAssets/Input/Aktions/IA_Jump`
  (params (ActionValue :type Boolean) (ElapsedSeconds :type "Float (double-precision)") (TriggeredSeconds :type "Float (double-precision)") (InputAction :type "InputAction Object Reference" :default "/Game/GameAssets/Input/Aktions/IA_Jump.IA_Jump"))
  (:`Started`
    (if (not (`self.IsAttacking`))
      (`self.Jump`)))
  (:`Completed`
    (`self.StopJumping`)))

(event `self.ReceiveTick`
  (params (DeltaSeconds :type "Float (single-precision)"))
  (`self.Update Animation`)
  (`self.FoodstepSound`)
  (`self.CheckHitBox`))

(event `CheckHitBox`
  (bind _returnvalue (`PaperFlipbookComponent.GetPlaybackPositionInFrames` (`self.Sprite`)))
  ;[1 1 1] AttackHitBox
  (if (== (`PaperFlipbookComponent.GetFlipbook` (`self.Sprite`)) "/Game/GameAssets/2DTestAsset/KnightAttack.KnightAttack")
    (if (or (== _returnvalue 3) (== _returnvalue 4))
      (for _array_element (`PrimitiveComponent.GetOverlappingActors` (`self.HitBoxFromAttack`) "/Script/Engine.Actor")
        (if (!= _array_element self)
          (`self.K2_DestroyActor` _array_element))))))

(event `FoodstepSound`
  (bind _returnvalue (`PaperFlipbookComponent.GetPlaybackPositionInFrames` (`self.Sprite`)))
  ;[1 1 1] Foodsteps
  (if (== (`PaperFlipbookComponent.GetFlipbook` (`self.Sprite`)) "/Game/GameAssets/2DTestAsset/KnightRun.KnightRun")
    (if (or (== _returnvalue 2) (== _returnvalue 6))
      (`/Engine/EditorBlueprintResources/StandardMacros.DoOnce` false :!label _label
        (:`Completed`
          (`GameplayStatics.PlaySoundAtLocation` "/Engine/VREditor/Sounds/UI/Click_on_Button.Click_on_Button" (`self.K2_GetActorLocation`) (struct) 1.0 1.0 0.0 null null null null)))
      (else
        (goto _label :!via `Reset`)))))

(event `self.Sprite.OnFinishedPlaying`
  ;[1 1 1] Return to Idle
  (set `self.IsAttacking` false)
  (if (`self.IsAttackInput`)
    (set `self.IsAttacking` true)
    (else
      (`PaperFlipbookComponent.SetLooping` (`self.Sprite`) true)))
  (`PaperFlipbookComponent.PlayFromStart` (`self.Sprite`)))

(event `TriggerFlash`
  (params (Multiplier :type "Float (single-precision)" :default 1.0) (Color :type "LinearColor Structure" :default (struct :`R` 1.0 :`A` 1.0)) (PlayRate :type "Float (single-precision)" :default 5.0))
  ;[1 1 1] TriggerFlash
  (`MaterialInstanceDynamic.SetScalarParameterValue` (`self.DynamicSpriteMaterial`) "FlashMultiplier" Multiplier)
  (`MaterialInstanceDynamic.SetVectorParameterValue` (`self.DynamicSpriteMaterial`) "FlashColor" Color)
  (`TimelineComponent.SetPlayRate` (`self.TimelineFlashMultiplayer`) PlayRate)
  (bind (_direction _alpha) (`Timeline|TimelineFlashMultiplayer` :!via `PlayFromStart`)
    (:`Update`
      (`MaterialInstanceDynamic.SetScalarParameterValue` (`self.DynamicSpriteMaterial`) "FlashMultiplier" (`KismetMathLibrary.Lerp` 0.0 Multiplier _alpha)))))

(fn `Update Animation`
  (bind _returnvalue_x (`KismetMathLibrary.BreakVector` (`self.GetVelocity`)))
  (bind (_returnvalue_x_2 _returnvalue_y _returnvalue_z) (`KismetMathLibrary.BreakVector` (`self.GetVelocity`)))
  (if (`NavMovementComponent.IsMovingOnGround` (`self.CharacterMovement`))
    (if (not (`self.IsAttacking`))
      ;[1 1 1] Run and Idle
      (if (< (`KismetMathLibrary.Abs` (`KismetMathLibrary.VSize` (`KismetMathLibrary.Conv_DoubleToVector` _returnvalue_x))) 0.1)
        (`PaperFlipbookComponent.SetFlipbook` (`self.Sprite`) "/Game/GameAssets/2DTestAsset/KnightIdle.KnightIdle")
        (else
          (`PaperFlipbookComponent.SetFlipbook` (`self.Sprite`) "/Game/GameAssets/2DTestAsset/KnightRun.KnightRun"))))
    (else
      ;[1 1 1] Jump Animation
      (if (< _returnvalue_z -50.0)
        (`PaperFlipbookComponent.SetFlipbook` (`self.Sprite`) "/Game/GameAssets/2DTestAsset/KnightJump.KnightJump")
        (else
          (`PaperFlipbookComponent.SetFlipbook` (`self.Sprite`) "/Game/GameAssets/2DTestAsset/KnightJump.KnightJump"))))))

(fn `UserConstructionScript`)